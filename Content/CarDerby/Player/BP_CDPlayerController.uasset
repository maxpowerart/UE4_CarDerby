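; Player controller for CarDerby that owns the toggling of the main menu.
; On BeginPlay it creates a WBP_Menu widget for player 0, stores it as MainMenu and adds it to the viewport hidden.
; The Menu input action flips that same widget between visible and hidden, so it is created only once.
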(event `self.ReceiveBeginPlay`
  ;[1 1 1] Create main menu widget
  (bind _returnvalue (`|CreateWidget` "/Game/CarDerby/UI/WBP_Menu.WBP_Menu_C" (`GameplayStatics.GetPlayerController` 0)))
  (set `self.MainMenu` _returnvalue)
  (`Widget.SetVisibility` _returnvalue "Hidden")
  (`UserWidget.AddToViewport` _returnvalue 0))

(event `InputAction|Menu` :paused true
  (params (Key :type "Key Structure"))
  (bind _mainmenu (`self.MainMenu`))
  ;[1 1 1] InputAction Menu
  (:`Pressed`
    (if (`Widget.IsVisible` (`self.MainMenu`))
      (`Widget.SetVisibility` _mainmenu "Hidden")
      (else
        (`Widget.SetVisibility` _mainmenu "Visible")))))

(fn `UserConstructionScript`)